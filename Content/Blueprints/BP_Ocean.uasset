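; BP_Ocean is an ocean actor that follows the player and acts as a kill plane for falling into the water.
; Each Tick it moves its static mesh under player 0's mesh in X and Y at world Z zero, as long as the player stays above it.
; Otherwise it sets IsDead to stop updating, prints a lose message and opens GameMapNone after a short delay.
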(event EventBeginPlay)

(event EventTick
  (params (DeltaSeconds :type Float%20%28single-precision%29))
  (bind _returnvalue (Game|GetPlayerCharacter 0))
  (bind _staticmesh (Variables|Default|GetStaticMesh))
  (bind _mesh (Variables|/Script/Engine.Character|GetMesh _returnvalue))
  (bind _returnvalue_2 (Transformation|GetWorldLocation _mesh))
  (if (not (Variables|Default|GetisDead))
    (if (> (.z _returnvalue_2) (.z (Transformation|GetWorldLocation _staticmesh)))
      (Transformation|SetWorldLocation _staticmesh (Math|Vector|MakeVector (.x _returnvalue_2) (.y _returnvalue_2) 0.0) false false)
      (else
        (Variables|Default|SetisDead true)
        (Development|PrintString "U LOSE")
        (Utilities|FlowControl|Delay 2.0)
        (Game|OpenLevel(byName) "GameMapNone")))))

(fn ConstructionScript)