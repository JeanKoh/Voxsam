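; World grid actor that holds a 3D array of block cells and spawns the starting blocks.
; On BeginPlay it fills the grid with empty cells, using nested structs to form the 3D array, with get and set helpers by X/Y/Z.
; It then spawns and places a BP_Block at each in-range StartingLocation, spaced 100 units from the actor's root.
; That spawn pass does not write the blocks into the grid.
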(event EventBeginPlay
  (CallFunction|Init3DGridArray)
  (CallFunction|InitBoxColliders))

(event Collision|EventActorBeginOverlap
  (params (OtherActor :type Actor%20Object%20Reference)))

(event EventTick
  (params (DeltaSeconds :type Float%20%28single-precision%29)))

(fn ConstructionScript)

(fn Init1DGridArray
  (for _index (range 0 (Utilities|Array|Get(acopy) (Variables|Default|GetGridSize) 2))
    (Utilities|Array|Add (LocalVariables|GetGridArray) (Utilities|Struct|MakeGridElement true "Empty")))
  (return (Utilities|Struct|Make1DGridArray (LocalVariables|GetGridArray))))

(fn Init2DGridArray
  (for _index (range 0 (Utilities|Array|Get(acopy) (Variables|Default|GetGridSize) 1))
    (bind _1dgridarray (CallFunction|Init1DGridArray))
    (Utilities|Array|Add (LocalVariables|Get1DGridArray) _1dgridarray))
  (return (Utilities|Struct|Make2DGridArray (LocalVariables|Get1DGridArray))))

(fn Init3DGridArray
  (for _index (range 0 (Utilities|Array|Get(acopy) (Variables|Default|GetGridSize)))
    (bind _2dgridarray (CallFunction|Init2DGridArray))
    (Utilities|Array|Add (Variables|Default|Get3D_WorldGrid) _2dgridarray)))

(fn GetGridElement
  (params (X :type Integer) (Y :type Integer) (Z :type Integer))
  (return (Utilities|Array|Get(acopy) (Utilities|Struct|Break1DGridArray (Utilities|Array|Get(acopy) (Utilities|Struct|Break2DGridArray (Utilities|Array|Get(acopy) (Variables|Default|Get3D_WorldGrid) X)) Y)) Z)))

(fn SetGridElement
  (params (X :type Integer) (Y :type Integer) (Z :type Integer) (Empty :type Boolean) (Block%20Type :type Name))
  (bind _3d_worldgrid (Variables|Default|Get3D_WorldGrid))
  (bind _item (Utilities|Array|Get(acopy) _3d_worldgrid X))
  (bind _1dgridarray (Utilities|Struct|Break2DGridArray _item))
  (bind _output_get (LocalVariables|SetTemp2DGrid _1dgridarray))
  (bind _output_get_2 (LocalVariables|SetTemp1DGrid (Utilities|Struct|Break1DGridArray (Utilities|Array|Get(acopy) _1dgridarray Y))))
  (Utilities|Array|SetArrayElem _output_get_2 Z (Utilities|Struct|MakeGridElement Empty Block%20Type))
  (Utilities|Array|SetArrayElem _output_get Y (Utilities|Struct|Make1DGridArray _output_get_2))
  (Utilities|Array|SetArrayElem _3d_worldgrid X (Utilities|Struct|Make2DGridArray _output_get)))

(fn InitBoxColliders
  (bind _gridsize (Variables|Default|GetGridSize))
  (for _array_element (Variables|Default|GetStartingLocations)
    (bind _isinrange (CallFunction|IntinRange (Math|Float|Truncate (.X (Math|Vector|BreakVector _array_element))) 0 (Utilities|Array|Get(acopy) _gridsize)))
    (bind _isinrange_2 (CallFunction|IntinRange (Math|Float|Truncate (.Y (Math|Vector|BreakVector _array_element))) 0 (Utilities|Array|Get(acopy) _gridsize 1)))
    (bind _isinrange_3 (CallFunction|IntinRange (Math|Float|Truncate (.Z (Math|Vector|BreakVector _array_element))) 0 (Utilities|Array|Get(acopy) _gridsize 2)))
    (if (Math|Boolean|ANDBoolean _isinrange _isinrange_2 _isinrange_3)
      (bind _returnvalue (Game|SpawnActorfromClass "/Game/Blueprints/BP_Block.BP_Block_C" (Math|Transform|MakeTransform (+ (Transformation|GetWorldLocation (Variables|Default|GetDefaultSceneRoot)) (Math|Vector|MakeVector (* (Math|Float|Truncate (.X (Math|Vector|BreakVector _array_element))) 1e+02) (* (Math|Float|Truncate (.Y (Math|Vector|BreakVector _array_element))) 1e+02) (* (Math|Float|Truncate (.Z (Math|Vector|BreakVector _array_element))) 1e+02))) "0, 0, 0" "1.000000,1.000000,1.000000") "Undefined" 0 0))
      (Default|PlaceBlock _returnvalue (Math|Transform|MakeTransform (+ (Transformation|GetWorldLocation (Variables|Default|GetDefaultSceneRoot)) (Math|Vector|MakeVector (* (Math|Float|Truncate (.X (Math|Vector|BreakVector _array_element))) 1e+02) (* (Math|Float|Truncate (.Y (Math|Vector|BreakVector _array_element))) 1e+02) (* (Math|Float|Truncate (.Z (Math|Vector|BreakVector _array_element))) 1e+02))) "0, 0, 0" "1.000000,1.000000,1.000000")))))

(fn IntinRange
  (params (Value :type Integer) (Lower :type Integer) (Upper :type Integer))
  (return (and (>= Value Lower) (<= Value Upper))))