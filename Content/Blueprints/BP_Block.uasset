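; BP_Block is a block actor that can be placed in the world, freezing its physics, or unplaced to simulate again.
; Once placed, grid toggling shows or hides six axis-side box colliders, switching them between query-only and no collision.
; Gaze hover sends held or info text to the HUD if the block can talk, and gaze off stops it.
; A hidden TextRender follows above the block each tick, but its display path is disconnected.
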(event EventBeginPlay
  (bind _block (Variables|Default|GetBlock))
  ;[1 1 1] Initialise Text Render Location
  (Variables|Default|SetTextRenderLocation (+ (Transformation|GetWorldLocation _block) (Math|Vector|MakeVector 0.0 0.0 (* (.z (Transformation|GetWorldScale _block)) (Variables|Default|GetTextOffset)))))
  ;[1 1 1] Set Text Render Location
  (Transformation|SetWorldLocation (Variables|Default|GetTextRender) (Variables|Default|GetTextRenderLocation) false false))

(event Collision|EventActorBeginOverlap
  (params (OtherActor :type Actor%20Object%20Reference)))

(event EventTick
  (params (DeltaSeconds :type Float%20%28single-precision%29))
  (bind _block (Variables|Default|GetBlock))
  ;[1 1 1] Initialise Text Render Location
  (Variables|Default|SetTextRenderLocation (+ (Transformation|GetWorldLocation _block) (Math|Vector|MakeVector 0.0 0.0 (* (.z (Transformation|GetWorldScale _block)) (Variables|Default|GetTextOffset)))))
  ;[1 1 1] Set Text Render Location
  (Transformation|SetWorldLocation (Variables|Default|GetTextRender) (Variables|Default|GetTextRenderLocation) false false))

(event EventGazeOff
  ;[1 1 1] When player takes gaze off
  (Development|SetHiddeninGame (Variables|Default|GetTextRender) true false)
  (Class|BPIBlock|StopTexttoHUD(Message) (Utilities|GetHUD)))

(fn ConstructionScript
  (Development|SetHiddeninGame (Variables|Default|GetTextRender) true false))

(fn GetAngle
  (params (Vector1 :type Vector) (Vector2 :type Vector))
  (return (Class|KismetMathLibrary|DegAcos (/ (Math|Vector|DotProduct Vector1 Vector2) (* (Math|Vector|VectorLength Vector1) (Math|Vector|VectorLength Vector2))))))

(fn GetNormalVector
  (params (Vector1 :type Vector) (Vector2 :type Vector))
  (return (/ (Math|Vector|CrossProduct Vector1 Vector2) (* (Math|Vector|VectorLength Vector1) (Math|Vector|VectorLength Vector2)))))

(fn PlaceBlock
  (params (Location :type Transform))
  (bind _block (Variables|Default|GetBlock))
  (Variables|Default|SetPlaced true)
  (Transformation|SetWorldTransform _block Location false false)
  (Physics|SetSimulatePhysics _block false))

(fn ToggleGridColliders
  (params (On :type Boolean))
  (if (Variables|Default|GetPlaced)
    (if On
      (LocalVariables|SetCollisionEnum "QueryOnly")
      (else
        (LocalVariables|SetCollisionEnum "NoCollision")))
    (Utilities|FlowControl|Sequence
      (:then_0
        (CallFunction|ToggleCollider (Variables|Default|GetBoxNegX) (LocalVariables|GetCollisionEnum)))
      (:then_1
        (CallFunction|ToggleCollider (Variables|Default|GetBoxPosX) (LocalVariables|GetCollisionEnum)))
      (:then_2
        (CallFunction|ToggleCollider (Variables|Default|GetBoxNegY) (LocalVariables|GetCollisionEnum)))
      (:then_3
        (CallFunction|ToggleCollider (Variables|Default|GetBoxPosY) (LocalVariables|GetCollisionEnum)))
      (:then_4
        (CallFunction|ToggleCollider (Variables|Default|GetBoxNegZ) (LocalVariables|GetCollisionEnum)))
      (:then_5
        (CallFunction|ToggleCollider (Variables|Default|GetBoxPosZ) (LocalVariables|GetCollisionEnum))))))

(fn ToggleCollider
  (params (Collider :type Primitive%20Component%20Object%20Reference) (CollisionEnum :type ECollisionEnabled%20Enum))
  (Collision|SetCollisionEnabled Collider CollisionEnum)
  (Development|SetHiddeninGame Collider (Utilities|Enum|Equal(Enum) CollisionEnum "NoCollision") false))

(fn UnplaceBlock
  (Variables|Default|SetPlaced false)
  (Physics|SetSimulatePhysics (Variables|Default|GetBlock) true))

(fn DisplayTextRender
  (params (PlayerLocation :type Vector) (LocationOfText :type Vector))
  (bind _textrender (Variables|Default|GetTextRender))
  (bind _textrender_2 (Variables|Default|GetTextRender))
  (bind _textrender_3 (Variables|Default|GetTextRender))
  (bind _returnvalue (Transformation|GetWorldLocation _textrender))
  (bind _returnvalue_2 (- PlayerLocation _returnvalue))
  (bind _returnvalue_3 (Math|Vector|VectorLength _returnvalue_2))
  (bind _returnvalue_4 (/ _returnvalue_3 3e+02))
  (if (Rendering|IsVisible (Variables|Default|GetTextRender))
    _
    (else
      (Development|SetHiddeninGame _textrender_2 false false)))
  (Transformation|SetWorldRotation _textrender_2 (Math|Rotator|MakeRotfromX _returnvalue_2) false false)
  (Variables|Default|SetTextRenderLocation LocationOfText)
  (Transformation|SetWorldScale3D _textrender_3 (Math|Vector|MakeVector _returnvalue_4 _returnvalue_4 _returnvalue_4))
  (Rendering|Components|TextRender|SetText _textrender_3 (Utilities|Text|ToText(String) (Variables|Default|GetCurrentlyDisplayedText)))
  (return))

(fn GazeHover
  (params (ObjectHeld? :type Boolean) (PlayerLocation :type Vector) (LocationOfText :type Vector))
  (if (Variables|Default|GetCanBlockTalk?)
    (if ObjectHeld?
      (Variables|Default|SetCurrentlyDisplayedText (Variables|Default|GetHeldByPlayer))
      (else
        (Variables|Default|SetCurrentlyDisplayedText (Variables|Default|GetInformation))))
    (Class|BPIBlock|TexttoHUD(Message) (Utilities|GetHUD) (Variables|Default|GetCurrentlyDisplayedText) (Variables|Default|GetTextRenderLocation)))
  (return true))

(fn GetPlacedBlock
  (return true (Variables|Default|GetPlaced)))

(fn SetPlacedBlock
  (params (Placed :type Boolean) (Location :type Vector))
  (bind _block (Variables|Default|GetBlock))
  (if Placed
    (Transformation|SetWorldTransform _block (Math|Conversions|ToTransform(Vector) Location) false false)
    (Transformation|SetActorLocation Location false false))
  (Variables|Default|SetPlaced Placed)
  (Physics|SetSimulatePhysics _block (not Placed))
  (return true))

(fn ToggleGrid
  (params (Toggle :type Boolean))
  (CallFunction|ToggleGridColliders Toggle)
  (return true))