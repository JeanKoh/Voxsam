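; BP_Projectile is a monster AI projectile that can home in on a block and explodes on impact.
; The HomingMissle event casts its target to BP_Block and sets that block's component as the projectile movement's homing target with strong acceleration, printing debug text on failure.
; The first collision hit spawns an explosion particle at the sphere and destroys the actor, without applying any damage itself.
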(event OnComponentHit(CollisionComponent)
  (params (HitComponent :type Primitive%20Component%20Object%20Reference) (OtherActor :type Actor%20Object%20Reference) (OtherComp :type Primitive%20Component%20Object%20Reference) (NormalImpulse :type Vector :default "0, 0, 0") (Hit :type Hit%20Result%20Structure%20%28by%20ref%29))
  ;[1 1 1] Emitter
  (Utilities|FlowControl|DoOnce false
    (:Completed
      (Effects|SpawnEmitteratLocation "/Game/StarterContent/Particles/P_Explosion.P_Explosion" (Transformation|GetWorldLocation (Variables|MyProjectile|GetSphere)))
      (Actor|DestroyActor))))

(event Custom|HomingMissle
  (params (target%20to%20hit :type Actor%20Object%20Reference))
  (bind _projectile (Variables|MyProjectile|GetProjectile))
  ;[1 1 1] Set Homing Missile
  (if (Utilities|IsValid target%20to%20hit)
    (bind _asbp_block (Utilities|Casting|CastToBP_Block target%20to%20hit)
      (:then
        (Variables|/Script/Engine.ProjectileMovementComponent|SetHomingTargetComponent _projectile (Variables|/Game/FirstPersonBP/Blueprints/BP_Block.BP_Block_C|GetBlock _asbp_block))
        (Variables|/Script/Engine.ProjectileMovementComponent|SetbIsHomingProjectile _projectile true)
        (Variables|/Script/Engine.ProjectileMovementComponent|SetHomingAccelerationMagnitude _projectile 2.5e+04))
      (:CastFailed
        (Development|PrintString "FAIL CAST")))
    (else
      (Development|PrintString "invalid..."))))

(fn ConstructionScript)